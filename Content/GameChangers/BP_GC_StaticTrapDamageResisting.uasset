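; Game changer pickup that temporarily makes all BP_StaticTrap actors deal no damage.
; On sphere overlap it hides itself, and if the overlapping actor is BP_ThirdPersonCharacter it calls PlayerAbsorb.
; PlayerAbsorb caches each trap's Damage in a map keyed by actor, zeroes it, and waits for Duration.
; It then restores the cached values, clears the map and calls Dispose.
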(event `self.SphereCollision.OnComponentBeginOverlap`
  (params (OverlappedComponent :type "PrimitiveComponent Object Reference") (OtherActor :type "Actor Object Reference") (OtherComp :type "PrimitiveComponent Object Reference") (OtherBodyIndex :type Integer) (bFromSweep :type Boolean) (SweepResult :type "HitResult Structure (by ref)"))
  (`self.SetActorHiddenInGame` true)
  (`KismetSystemLibrary.PrintText` "StaticTrapDamageResisting Started")
  (bind _asbp_third_person_character (cast `/Game/ThirdPerson/Blueprints/BP_ThirdPersonCharacter` OtherActor))
  (`self.PlayerAbsorb` _asbp_third_person_character))

(event `/Game/Interfaces/BPI_PlayerAbsorbing.PlayerAbsorb`
  (params (Player :type "/Game/ThirdPerson/Blueprints/BP_ThirdPersonCharacter Object Reference"))
  (bind _outactors (`GameplayStatics.GetAllActorsOfClass` "/Game/Traps/Static/BP_StaticTrap.BP_StaticTrap_C"))
  (for _array_element _outactors
    ;[1 1 1] Note Original Damage of all MoveableTraps
    (`BlueprintMapLibrary.Map_Add` (`self.OriginalDamageHashMap`) _array_element (`/Game/Traps/BP_Parent_Trap.Damage` _array_element))
    ;[1 1 1] Set Damage = 0
    (set `/Game/Traps/BP_Parent_Trap.Damage` 0.0 _array_element))
  ;[1 1 1] Delay
  (`KismetSystemLibrary.Delay` (`self.Duration`))
  ;[1 1 1] Set Original Damage back
  (bind _keys (`BlueprintMapLibrary.Map_Keys` (`self.OriginalDamageHashMap`)))
  (for _array_element_2 _keys
    (bind _asbp_static_trap (cast `/Game/Traps/Static/BP_StaticTrap` _array_element_2))
    (set `/Game/Traps/BP_Parent_Trap.Damage` (`BlueprintMapLibrary.Map_Find` (`self.OriginalDamageHashMap`) _asbp_static_trap) _asbp_static_trap))
  ;[1 1 1] Clear Hash Map
  (`BlueprintMapLibrary.Map_Clear` (`self.OriginalDamageHashMap`))
  (`/Game/Interfaces/BPI_Disposable.Dispose`)
  (`KismetSystemLibrary.PrintText` "StaticTrapDamageResisting Finished"))

(fn `UserConstructionScript`
  (`parent.UserConstructionScript`))