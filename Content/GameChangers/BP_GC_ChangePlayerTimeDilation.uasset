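; Game-changer pickup that temporarily changes the player character's time dilation when touched.
; Overlapping Sphere1 with BP_ThirdPersonCharacter triggers PlayerAbsorb, which hides the actor and sets that character's CustomTimeDilation to SlowDownMultiplier.
; After Duration it resets the dilation to 1.0 and calls Dispose; the construction script only runs the parent's.
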(event `self.Sphere1.OnComponentBeginOverlap`
  (params (OverlappedComponent :type "PrimitiveComponent Object Reference") (OtherActor :type "Actor Object Reference") (OtherComp :type "PrimitiveComponent Object Reference") (OtherBodyIndex :type Integer) (bFromSweep :type Boolean) (SweepResult :type "HitResult Structure (by ref)"))
  (bind _asbp_third_person_character (cast `/Game/ThirdPerson/Blueprints/BP_ThirdPersonCharacter` OtherActor))
  (`self.PlayerAbsorb` _asbp_third_person_character))

(event `/Game/Interfaces/BPI_PlayerAbsorbing.PlayerAbsorb`
  (params (Player :type "/Game/ThirdPerson/Blueprints/BP_ThirdPersonCharacter Object Reference"))
  (`self.SetActorHiddenInGame` true)
  (set `Actor.CustomTimeDilation` (`self.SlowDownMultiplier`) Player)
  (`KismetSystemLibrary.Delay` (`self.Duration`))
  (set `Actor.CustomTimeDilation` 1.0 Player)
  (`self.Dispose`))

(fn `UserConstructionScript`
  (`parent.UserConstructionScript`))