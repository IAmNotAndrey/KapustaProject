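; BP_GC_Random is a game changer pickup that resolves into a randomly chosen effect when the third-person character touches it.
; On sphere overlap, PlayerAbsorb hides the actor and spawns a random class from ClassesMayBecome.
; It immediately forwards the absorb call and player to the spawned actor, then disposes of itself, acting purely as a proxy.
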(event `self.Sphere1.OnComponentBeginOverlap`
  (params (OverlappedComponent :type "PrimitiveComponent Object Reference") (OtherActor :type "Actor Object Reference") (OtherComp :type "PrimitiveComponent Object Reference") (OtherBodyIndex :type Integer) (bFromSweep :type Boolean) (SweepResult :type "HitResult Structure (by ref)"))
  (bind _asbp_third_person_character (cast `/Game/ThirdPerson/Blueprints/BP_ThirdPersonCharacter` OtherActor))
  (`self.PlayerAbsorb` _asbp_third_person_character))

(event `/Game/Interfaces/BPI_PlayerAbsorbing.PlayerAbsorb`
  (params (Player :type "/Game/ThirdPerson/Blueprints/BP_ThirdPersonCharacter Object Reference"))
  (`self.SetActorHiddenInGame` true)
  (bind _returnvalue (`|SpawnActorFromClass` (`KismetArrayLibrary.Array_Random` (`self.ClassesMayBecome`)) (`KismetMathLibrary.MakeTransform` (0.0 0.0 0.0)) "Undefined" "MultiplyWithRoot" null null))
  (`/Game/Interfaces/BPI_PlayerAbsorbing.PlayerAbsorb` _returnvalue Player)
  (`/Game/Interfaces/BPI_Disposable.Dispose`))

(fn `UserConstructionScript`
  (`parent.UserConstructionScript`))