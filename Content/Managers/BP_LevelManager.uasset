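; Level manager that registers itself with the game instance and drives a PCG trap field of traps, heals and game changers.
; On BeginPlay it reads a shared-params DataTable, sets PCG density, regenerates, then after a short delay randomizes spawned actors' stats within ranges.
; NewLevel maps difficulty through a sigmoid to point density, reseeds and regenerates, optionally spawns a healer or finish point, and teleports the player to start.
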(event Custom|Event%20NewLevel
  (params (IsHarder :type Boolean) (IsFinishLevel :type Boolean) (Player :type BP%20Third%20Person%20Character%20Object%20Reference))
  (Utilities|FlowControl|Sequence
    (:then_0
      ;[1 1 1] Set density of points on PCG. The higher difficulty, the more points
      (bind _asbp_game_instance (CallFunction|GetGameInstance))
      (bind _result (CallFunction|GetCustomSigmoid (Math|Conversions|ToFloat(Integer) (Variables|/Game/Instances/BP_GameInstance.BP_GameInstance_C|GetLevelDifficulty _asbp_game_instance))))
      (Variables|/Game/Traps/BP_PCG_TrapField.BP_PCG_TrapField_C|SetPointsPerSquaredMeterPCG (Variables|Default|GetTrapField) _result))
    (:then_1
      (CallFunction|SetRandomSeedPCG))
    (:then_2
      (CallFunction|UpdatePCG))
    (:then_3
      (if IsHarder
        (CallFunction|SpawnHeal)))
    (:then_4
      (if IsFinishLevel
        (CallFunction|SpawnFinishPoint)))
    (:then_5
      (CallFunction|TeleportPlayertoStartPoint Player))))

(event Custom|MultiplyTrapSpeed
  (params (Multiplier :type Float%20%28double-precision%29))
  ;[1 1 1] Multiply Moveable Traps speed
  (bind _outactors (Actor|GetAllActorsOfClass "/Game/Traps/Moveable/BP_MoveableTrap.BP_MoveableTrap_C"))
  (for _array_element _outactors
    (Variables|/Game/Traps/Moveable/BP_MoveableTrap.BP_MoveableTrap_C|SetLoopTime _array_element (* (Variables|/Game/Traps/Moveable/BP_MoveableTrap.BP_MoveableTrap_C|GetLoopTime _array_element) Multiplier))))

(event Custom|Set_GameChangers_DensityBounds_PCG
  (params (Value :type Vector%202D%20Structure))
  (bind (_x _y) (Math|Vector2D|BreakVector2D Value))
  (bind _trapfield (Variables|Default|GetTrapField))
  ;[1 1 1] Set PCG Parameters
  (Variables|/Game/Traps/BP_PCG_TrapField.BP_PCG_TrapField_C|SetGameChangersDensity_LowerBound _trapfield _x)
  (Variables|/Game/Traps/BP_PCG_TrapField.BP_PCG_TrapField_C|SetGameChangersDensity_UpperBound _trapfield _y))

(event Custom|SetGameChangersDuration
  (params (Values :type Vector%202D%20Structure))
  (bind (_x _y) (Math|Vector2D|BreakVector2D Values))
  (bind _outactors (Actor|GetAllActorsOfClass "/Game/GameChangers/BP_Parent_GameChanger.BP_Parent_GameChanger_C"))
  (for _array_element _outactors
    (Variables|/Game/GameChangers/BP_Parent_GameChanger.BP_Parent_GameChanger_C|SetDuration _array_element (Math|Random|RandomFloatinRange _x _y))))

(event Custom|SetTrapSpeed
  (params (Values :type Vector%202D%20Structure))
  (bind (_x _y) (Math|Vector2D|BreakVector2D Values))
  ;[1 1 1] Set Moveable Traps speed
  (bind _outactors (Actor|GetAllActorsOfClass "/Game/Traps/Moveable/BP_MoveableTrap.BP_MoveableTrap_C"))
  (for _array_element _outactors
    (Variables|/Game/Traps/Moveable/BP_MoveableTrap.BP_MoveableTrap_C|SetLoopTime _array_element (Math|Random|RandomFloatinRange _x _y))))

(event Custom|SetTrapDamage
  (params (Values :type Vector%202D%20Structure))
  (bind (_x _y) (Math|Vector2D|BreakVector2D Values))
  ;[1 1 1] Set Traps Damage
  (bind _outactors (Actor|GetAllActorsOfClass "/Game/Traps/BP_Parent_Trap.BP_Parent_Trap_C"))
  (for _array_element _outactors
    (Variables|/Game/Traps/BP_Parent_Trap.BP_Parent_Trap_C|SetDamage _array_element (Math|Random|RandomFloatinRange _x _y))))

(event Custom|SetHealerHP
  (params (Values :type Vector%202D%20Structure))
  (bind (_x _y) (Math|Vector2D|BreakVector2D Values))
  ;[1 1 1] Set Healers Add HP
  (bind _outactors (Actor|GetAllActorsOfClass "/Game/Healers/BP_Parent_Heal.BP_Parent_Heal_C"))
  (for _array_element _outactors
    (Variables|/Game/Healers/BP_Parent_Heal.BP_Parent_Heal_C|SetAddHP _array_element (Math|Random|RandomFloatinRange _x _y))))

(event Custom|SetPointsPerSquaredMeter
  (params (Value :type Float%20%28double-precision%29))
  ;[1 1 1] Set PCG Parameters
  (Variables|/Game/Traps/BP_PCG_TrapField.BP_PCG_TrapField_C|SetPointsPerSquaredMeterPCG (Variables|Default|GetTrapField) Value))

(event Custom|Set_Heals_DensityBounds_PCG
  (params (Values :type Vector%202D%20Structure))
  (bind (_x _y) (Math|Vector2D|BreakVector2D Values))
  (bind _trapfield (Variables|Default|GetTrapField))
  ;[1 1 1] Set PCG Parameters
  (Variables|/Game/Traps/BP_PCG_TrapField.BP_PCG_TrapField_C|SetHealsDensity_LowerBound _trapfield _x)
  (Variables|/Game/Traps/BP_PCG_TrapField.BP_PCG_TrapField_C|SetHealsDensity_UpperBound _trapfield _y))

(event Custom|Set_Traps_DensityBounds_PCG
  (params (Values :type Vector%202D%20Structure))
  (bind (_x _y) (Math|Vector2D|BreakVector2D Values))
  (bind _trapfield (Variables|Default|GetTrapField))
  ;[1 1 1] Set PCG Parameters
  (Variables|/Game/Traps/BP_PCG_TrapField.BP_PCG_TrapField_C|SetTrapsDensity_LowerBound _trapfield _x)
  (Variables|/Game/Traps/BP_PCG_TrapField.BP_PCG_TrapField_C|SetTrapsDensity_UpperBound _trapfield _y))

(event EventBeginPlay
  (Utilities|FlowControl|Sequence
    (:then_0
      ;[1 1 1] Set GameManager `LevelManager` variable
      (bind _asbp_game_instance (CallFunction|GetGameInstance))
      (Variables|/Game/Instances/BP_GameInstance.BP_GameInstance_C|SetLevelManager _asbp_game_instance self))
    (:then_1
      ;[1 1 1] Get Data from SharaedParams DataTable
      (bind _returnvalue (Utilities|GetDataTableRow "/Game/Instances/DataTable_SharedParams.DataTable_SharedParams" "NewRow")
        (:then
          (CallFunction|SetPointsPerSquaredMeter (.PointsPerSquaredMeter (Utilities|Struct|BreakSCT_SharedParams _returnvalue)))
          (CallFunction|SetTrapsDensityBoundsPCG (.TrapsDensity (Utilities|Struct|BreakSCT_SharedParams _returnvalue)))
          (CallFunction|SetGameChangersDensityBoundsPCG (.GameChangersDensity (Utilities|Struct|BreakSCT_SharedParams _returnvalue)))
          (CallFunction|SetHealsDensityBoundsPCG (.HealsDensity (Utilities|Struct|BreakSCT_SharedParams _returnvalue)))
          (CallFunction|UpdatePCG)
          (Utilities|FlowControl|Delay 0.5)
          (CallFunction|SetTrapSpeed (.LoopTimeforMoveableTrap (Utilities|Struct|BreakSCT_SharedParams _returnvalue)))
          (CallFunction|SetTrapDamage (.TrapDamage (Utilities|Struct|BreakSCT_SharedParams _returnvalue)))
          (CallFunction|SetHealerHP (.HealHP (Utilities|Struct|BreakSCT_SharedParams _returnvalue)))
          (CallFunction|SetGameChangersDuration (.GameChangersDuration (Utilities|Struct|BreakSCT_SharedParams _returnvalue))))))))

(fn ConstructionScript)

(fn SetRandomSeedPCG
  ;[1 1 1] Set random seed to avoid same level
  (Variables|/Game/Traps/BP_PCG_TrapField.BP_PCG_TrapField_C|SetSeedPCG (Variables|Default|GetTrapField) (Math|Random|RandomIntegerinRange -2147483648 2147483647)))

(fn UpdatePCG
  ;[1 1 1] Update PCG
  (PCG|Generate (Variables|/Game/Traps/BP_PCG_TrapField.BP_PCG_TrapField_C|GetPCG_TrapField (Variables|Default|GetTrapField)) true))

(fn SpawnHeal
  ;[1 1 1] Spawn Heal if NewLevel harder than previous
  (Game|SpawnActorfromClass "/Game/Healers/BP_GarbageHealer.BP_GarbageHealer_C" (Math|Transform|MakeTransform (Variables|Coordinates|GetHealSpawnCoords) "0, 0, 0" "1.000000,1.000000,1.000000") "Undefined" "MultiplyWithRoot" 0 0))

(fn SpawnFinishPoint
  ;[1 1 1] Spawn FinishPoint if it is FinishLevel
  (Game|SpawnActorfromClass "/Game/Finish/BP_FinishPoint.BP_FinishPoint_C" (Math|Transform|MakeTransform (Variables|Coordinates|GetFinishPointSpawnCoord) "0, 0, 0" "1.000000,1.000000,1.000000") "Undefined" "MultiplyWithRoot" 0 0))

(fn TeleportPlayertoStartPoint
  (params (Player :type BP%20Third%20Person%20Character%20Object%20Reference))
  ;[1 1 1] Teleport Player to StartPoint
  (Transformation|Teleport Player (Variables|Coordinates|GetStartPlayerPosition) "0, 0, 0"))