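; BP_Saw is a moving trap whose saw slides back and forth and damages what overlaps it.
; Two timelines form an endless ping-pong along the relative Y axis: one plays forward, the other plays in reverse, each restarting the other when finished.
; BeginPlay sets their play rate to the inverse of LoopTime.
; Overlaps on DamageCollision pass the other actor to DamagePlayerCharacter with the saw as damage causer.
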(event `self.ReceiveBeginPlay`
  (bind _saw (`self.Saw`))
  ;[1 1 1] Set play rate of timlines by speed
  (`TimelineComponent.SetPlayRate` (`self.Timeline`) (/ 1.0 (`self.LoopTime`)))
  (`TimelineComponent.SetPlayRate` (`self.Timeline_0`) (/ 1.0 (`self.LoopTime`)))
  ;[1 1 1] Looped ping-pong movement of the saw
  (bind (_direction _y_location) (`Timeline|Timeline` :!label _label)
    (:`Update`
      (`SceneComponent.K2_SetRelativeLocation` _saw (`KismetMathLibrary.MakeVector` 0.0 _y_location) false false))
    (:`Finished`
      (bind (_direction_2 _y_location_2) (`Timeline|Timeline_0` :!via `ReverseFromEnd`)
        (:`Update`
          (`SceneComponent.K2_SetRelativeLocation` _saw (`KismetMathLibrary.MakeVector` 0.0 _y_location_2) false false))
        (:`Finished`
          (goto _label :!via `PlayFromStart`))))))

(event `self.DamageCollision.OnComponentBeginOverlap`
  (params (OverlappedComponent :type "PrimitiveComponent Object Reference") (OtherActor :type "Actor Object Reference") (OtherComp :type "PrimitiveComponent Object Reference") (OtherBodyIndex :type Integer) (bFromSweep :type Boolean) (SweepResult :type "HitResult Structure (by ref)"))
  ;[1 1 1] Damage
  (`self.Damage Player Character` OtherActor self))

(fn `UserConstructionScript`
  (`parent.UserConstructionScript`))