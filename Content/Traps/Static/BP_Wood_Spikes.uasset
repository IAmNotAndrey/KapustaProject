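; BP_Wood_Spikes is a static trap of wooden spikes that damages the player and can itself be destroyed.
; An overlap on DamageCollision passes the overlapping actor to DamagePlayerCharacter, with the trap as damage causer.
; GetDamage subtracts incoming damage from HP and calls Dispose when the result would be zero or less.
; The construction script only calls its parent version.
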(event `self.DamageCollision.OnComponentBeginOverlap`
  (params (OverlappedComponent :type "PrimitiveComponent Object Reference") (OtherActor :type "Actor Object Reference") (OtherComp :type "PrimitiveComponent Object Reference") (OtherBodyIndex :type Integer) (bFromSweep :type Boolean) (SweepResult :type "HitResult Structure (by ref)"))
  (`self.Damage Player Character` OtherActor self))

(event `/Game/Interfaces/BPI_Damageable.Get Damage`
  (params (Damage :type "Float (double-precision)"))
  (bind _returnvalue (- (`self.HP`) Damage))
  (if (> _returnvalue 0.0)
    (set `self.HP` _returnvalue)
    (else
      (`/Game/Interfaces/BPI_Disposable.Dispose`))))

(fn `UserConstructionScript`
  (`parent.UserConstructionScript`))